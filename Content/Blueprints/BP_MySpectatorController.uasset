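; BP_MySpectatorController is a player controller that shows the HUD and handles mouse hover over hex tiles.
; On BeginPlay it creates WBP_HUD, stores the reference and adds it to the viewport.
; Every Tick it traces under the cursor for WorldDynamic objects and calls SetHovered(true) on any BP_HexTile hit.
; It never clears the hovered state itself.
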(event EventBeginPlay
  (bind _returnvalue (UserInterface|CreateWidget "/Game/UI/WBP_HUD.WBP_HUD_C" self))
  (bind _output_get (Variables|Default|SetHUDRef _returnvalue))
  (UserInterface|Viewport|AddtoViewport _output_get 0))

(event EventTick
  (params (DeltaSeconds :type Float%20%28single-precision%29))
  (bind _array (Utilities|Array|MakeArray "ObjectTypeQuery2"))
  (bind (_hitresult _returnvalue) (Class|PlayerController|GetHitResultUnderCursorforObjects _array false))
  (if _returnvalue
    (bind _asbp_hex_tile_2 (Utilities|Casting|CastToBP_HexTile (.HitActor (Collision|BreakHitResult _hitresult))))
    (Default|SetHovered _asbp_hex_tile_2 true)))

(fn ConstructionScript)